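; BP_AIClient is the AI logic for a client character that orders a random recipe at a bar.
; An Init event, meant to be called from BP_Client, runs the BT_Client behavior tree and seeds its Blackboard with the bar location, client state and chosen recipe.
; TakeRandomRecipe picks that recipe uniformly from the AllRecipes list.
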(event Custom|Init
  (AI|RunBehaviorTree "/Game/_ProjetFiles/_Core/AI/BT_Client.BT_Client")
  (AI|Components|Blackboard|SetValueasObject (AI|GetBlackboard 0) (Utilities|Name|MakeLiteralName "barLocation") (Variables|Default|GetbarLocation))
  (AI|Components|Blackboard|SetValueasEnum (AI|GetBlackboard 0) (Utilities|Name|MakeLiteralName "state") (Variables|Default|GetclientState))
  (bind _output_get (Variables|Default|SetrecipeChoisen (CallFunction|TakeRandomRecipe)))
  (AI|Components|Blackboard|SetValueasObject (AI|GetBlackboard 0) (Utilities|Name|MakeLiteralName "recipe") _output_get))

(event EventBeginPlay)

(fn ConstructionScript)

(fn TakeRandomRecipe
  (bind _allrecipes (Variables|Default|GetAllRecipes))
  (bind _recipes (Variables|/Game/_ProjetFiles/_Core/Datas/TablesRecipes/BPDA_TableRecipes.BPDA_TableRecipes_C|Getrecipes _allrecipes))
  (return (Utilities|Array|Get(acopy) _recipes (Math|Random|RandomIntegerinRange 0 (- (Utilities|Array|Length _recipes) 1)))))