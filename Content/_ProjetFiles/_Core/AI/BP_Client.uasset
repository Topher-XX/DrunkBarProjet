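; BP_Client is an AI client that accepts a drink glass from the player and judges it against its chosen recipes.
; On interact, it attaches the held glass and compares ingredient quantities within a tolerance, accepting the first recipe with errors below a limit.
; A correct order pays money through the player controller's ACS_Money component.
; Either outcome updates the client's Blackboard state and destroys the glass.
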(event Custom|OnInteract
  (params (isInteract :type Boolean) (hand :type Scene%20Component%20Object%20Reference))
  (bind _returnvalue (Game|GetPlayerController 0))
  (bind _aiclient (Variables|Default|GetaiClient))
  (bind _returnvalue_2 (Actor|GetComponentbyClass _returnvalue "/Game/_ProjetFiles/_Core/ACS/ACS_Money.ACS_Money_C"))
  ;[0 0 1] On Interact
  ;;[1 1 1] Take glass
  (bind _asbp_glass (Utilities|Casting|CastToBP_Glass (Components|GetOwner (Components|GetChildComponent hand 0)))
    (:then
      (Variables|Default|Setglass _asbp_glass)
      (Transformation|AttachComponentToComponent _asbp_glass (Variables|Collision|GetCapsuleComponent) "None" "SnapToTarget" "SnapToTarget" "KeepRelative" true)
      ;;[1 1 1] Check ingredient and quantity
      (bind _array_element (Utilities|Array|ForEachLoopwithBreak (Variables|/Game/_ProjetFiles/_Core/AI/BP_AIClient.BP_AIClient_C|GetrecipeChoisen (Variables|Default|GetaiClient)) :!label _label) ; For each recipes
        (:LoopBody
          (bind _output_get (Variables|Default|SetcurrentRecipeCheck _array_element))
          (bind _keys (Utilities|Map|Keys (Variables|/Game/_ProjetFiles/_Core/Datas/BPDA_RecipeTemplate.BPDA_RecipeTemplate_C|Getingredient _output_get)))
          (for _array_element_2 _keys ; For each ingredients
            (if (.ReturnValue (Utilities|Map|Find (Variables|/Game/_ProjetFiles/_Core/EnvirronementElements/Templates/BP_Takable.BP_Takable_C|Getingredient (Variables|Default|Getglass)) _array_element_2)) ; This ingredient is in the glass
              (if (Math|Float|NearlyEqual(Float) (.Value (Utilities|Map|Find (Variables|/Game/_ProjetFiles/_Core/EnvirronementElements/Templates/BP_Takable.BP_Takable_C|Getingredient (Variables|Default|Getglass)) _array_element_2)) (.Value (Utilities|Map|Find (Variables|/Game/_ProjetFiles/_Core/Datas/BPDA_RecipeTemplate.BPDA_RecipeTemplate_C|Getingredient (Variables|Default|GetcurrentRecipeCheck)) _array_element_2)) (Variables|Default|GetingredientsErrorTolerance)) ; The ingredient quantity is correct
                (bind _result (Math|Integer|IncrementInt (Variables|Default|GetnbGood))
                  (:%20%20
                    (Variables|Default|SetnbGood _result)))
                (else
                  (bind _result_2 (Math|Integer|IncrementInt (Variables|Default|GetnbBad) :!label _label_2)
                    (:%20%20
                      (Variables|Default|SetnbBad _result_2)))))
              (else
                (goto _label_2))))
          (if (< (Variables|Default|GetnbBad) (Variables|Default|GetmaxError))
            (Variables|Default|SetcorrectOrder true)
            (goto _label Break)
            (else
              (Variables|Default|SetcorrectOrder false)
              (Variables|Default|SetnbBad 0)
              (Variables|Default|SetnbGood 0))))
        (:Completed
          ;;[1 1 1] check is order is correct
          (if (Variables|Default|GetcorrectOrder)
            (Development|PrintString (Utilities|String|Append "Happy : " (Utilities|String|ToString(Integer) (Variables|Default|GetnbBad))))
            (Utilities|IsValid _returnvalue_2
              (:Is%20Valid
                (Default|GiveMoneyEvent _returnvalue_2 (Math|Float|MapRangeClamped (Variables|Default|GetpercentMoneyToGive) 0.0 1.0 (Variables|/Game/_ProjetFiles/_Core/Datas/BPDA_RecipeTemplate.BPDA_RecipeTemplate_C|GetminMoneyGain (Variables|Default|GetcurrentRecipeCheck)) (Variables|/Game/_ProjetFiles/_Core/Datas/BPDA_RecipeTemplate.BPDA_RecipeTemplate_C|GetmaxMoneyGain (Variables|Default|GetcurrentRecipeCheck)))))
              (:Is%20Not%20Valid
                (Development|PrintString "ACS Money not fund !")))
            (else
              (Development|PrintString (Utilities|String|Append "Sad : " (Utilities|String|ToString(Integer) (Variables|Default|GetnbBad))))))
          (bind _output_get_2 (Variables|/Game/_ProjetFiles/_Core/AI/BP_AIClient.BP_AIClient_C|SetclientState _aiclient "NewEnumerator3"))
          (AI|Components|Blackboard|SetValueasEnum (AI|GetBlackboard _aiclient) (Utilities|Name|MakeLiteralName "state") _output_get_2)
          (Actor|DestroyActor (Variables|Default|Getglass)))))
    (:CastFailed
      (Default|ResetInteractEvent (Variables|Default|GetACS_Interact)))))

(event EventBeginPlay
  ;[1 1 1] Init
  (EventDispatchers|BindEventtoOnInteract (Variables|Default|GetACS_Interact) (EventDispatchers|CreateEvent :!event Custom|OnInteract)))

(fn ConstructionScript)