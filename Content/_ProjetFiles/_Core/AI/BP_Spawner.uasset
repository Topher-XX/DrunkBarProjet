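; BP_Spawner is an actor that spawns one AI client when play begins.
; SpawnClient spawns the ClientPrefab at the spawner's transform and stores it, then casts its AI controller to BP_AIClient.
; It hands that controller a reference to itself plus the bar and outside locations, then calls Init on it.
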(event Custom|SpawnClient
  ;[1 1 1] Spawn Client
  (bind _returnvalue (Game|SpawnActorfromClass (Variables|Default|GetclientPrefab) (Transformation|GetActorTransform) "Undefined" "MultiplyWithRoot" 0 0))
  (bind _output_get (Variables|Default|Setclient _returnvalue))
  (bind _asbp_aiclient (Utilities|Casting|CastToBP_AIClient (AI|GetAIController _output_get)))
  (bind _output_get_2 (Variables|Default|SetaiClient _asbp_aiclient))
  (Variables|/Game/_ProjetFiles/_Core/AI/BP_AIClient.BP_AIClient_C|Setspawner _output_get_2 self)
  (Variables|/Game/_ProjetFiles/_Core/AI/BP_AIClient.BP_AIClient_C|SetbarLocation (Variables|Default|GetaiClient) (Variables|Default|GetbarLocation))
  (Variables|/Game/_ProjetFiles/_Core/AI/BP_AIClient.BP_AIClient_C|Setoutside (Variables|Default|GetaiClient) (Variables|Default|GetoutsideLocation))
  (Default|Init (Variables|Default|GetaiClient)))

(event EventBeginPlay
  ;[1 1 1] Spawn client on start
  (CallFunction|SpawnClient))

(fn ConstructionScript)