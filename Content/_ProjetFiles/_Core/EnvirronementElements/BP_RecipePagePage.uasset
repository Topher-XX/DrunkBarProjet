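; BP_RecipePagePage is an interactable recipe page that displays a recipe through a widget component.
; On BeginPlay it passes its Recipe to the WBP_Recipe widget and initializes it.
; It extends the parent's interact and cancel events to disable the widget's collision on interaction and restore query and physics collision on cancel.
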(event EventOnInteract
  (params (IsInteract :type Boolean) (hand :type Scene%20Component%20Object%20Reference))
  (|CallParentFunction IsInteract hand)
  (Collision|SetCollisionEnabled (Variables|Default|GetWidget) "NoCollision"))

(event EventOnCancel
  (|CallParentFunction)
  (Collision|SetCollisionEnabled (Variables|Default|GetWidget) "QueryAndPhysics"))

(event EventBeginPlay
  (|CallParentFunction)
  (bind _aswbp_recipe (Utilities|Casting|CastToWBP_Recipe (UserInterface|GetWidget (Variables|Default|GetWidget))))
  (Variables|/Game/_ProjetFiles/_Core/Widgets/WBP_Recipe.WBP_Recipe_C|Setrecipe _aswbp_recipe (Variables|Default|GetRecipe))
  (Default|Init _aswbp_recipe))

(fn ConstructionScript)