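; BP_GlassCupboard is an interactable cupboard that hands the player a glass or takes one back.
; Its OnInteract override calls the parent, then spawns a BP_Glass and snaps it to the Hand component with mesh collision disabled if the hand is empty.
; If the hand is occupied, it destroys the first attached item's actor only when that casts to BP_Glass.
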(event EventBeginPlay
  (|CallParentFunction) ; This node is disabled and will not be called.\nDrag off pins to build functionality.
)

(event EventOnInteract
  (params (IsInteract :type Boolean) (hand :type Scene%20Component%20Object%20Reference))
  ;[0 0 1] On Interact
  ;;[1 1 1] Add glass to the player's hand
  (|CallParentFunction IsInteract hand)
  (if (== (Class|SceneComponent|GetNumChildrenComponents hand) 0)
    (bind _returnvalue (Game|SpawnActorfromClass "/Game/_ProjetFiles/_Core/EnvirronementElements/ObjectsTakables/BP_Glass.BP_Glass_C" (Math|Transform|MakeTransform "0, 0, 0") "Undefined" "MultiplyWithRoot" 0 0))
    (Transformation|AttachComponentToComponent _returnvalue hand "None" "SnapToTarget" "SnapToTarget" "SnapToTarget" true)
    (Collision|SetCollisionEnabled (Variables|/Game/_ProjetFiles/_Core/EnvirronementElements/Templates/BP_InteractObject.BP_InteractObject_C|GetStaticMesh _returnvalue) "NoCollision")
    (else
      ;;[1 1 1] Remove Glass from the player's hand
      (bind _asbp_glass (Utilities|Casting|CastToBP_Glass (Components|GetOwner (Components|GetChildComponent hand 0)))) ; Check if we can change this not
      (Actor|DestroyActor _asbp_glass))))

(fn ConstructionScript
  (|CallParentFunction))