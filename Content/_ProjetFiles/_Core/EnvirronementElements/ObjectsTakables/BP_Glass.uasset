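; BP_Glass is a takable glass object that tracks the quantity of each ingredient transferred into it.
; On BeginPlay it binds to the add and remove events of its ACSTransfertIngredient component.
; Additions increase the stored quantity in the Ingredients map only for types already present as keys, while removal clears the whole map.
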(event Custom|AddIngrediant
  (params (ingredientType :type E_Ingredient%20Enum :default "NewEnumerator3") (quantity :type Float%20%28double-precision%29))
  (bind _ingredients (Variables|Default|Getingredients))
  (bind (_value _returnvalue) (Utilities|Map|Find _ingredients ingredientType))
  ;[1 1 1] Add ingrediant To the glass
  (if _returnvalue
    (Utilities|Map|Add _ingredients ingredientType (+ _value quantity))))

(event Custom|RemoveIngredients
  ;[1 1 1] Init Transfert Ingredient
  (Utilities|Map|Clear (Variables|Default|Getingredients)))

(event EventBeginPlay
  (bind _acs_transfertingredient (Variables|Default|GetACS_TransfertIngredient))
  ;[1 1 1] Init Transfert Ingredient
  (|CallParentFunction)
  (Utilities|IsValid _acs_transfertingredient
    (:Is%20Valid
      (EventDispatchers|BindEventtoOnAddIngredient _acs_transfertingredient (delegate Custom|AddIngrediant))
      (EventDispatchers|BindEventtoRemoveIngredients _acs_transfertingredient (delegate Custom|RemoveIngredients)))))

(fn ConstructionScript
  (|CallParentFunction))