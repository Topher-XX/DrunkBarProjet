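; BP_Shaker is a shaker, filed among takable objects, that accumulates a shake value while it holds ingredients.
; Its Shake event ignores input when the Ingredient list is empty.
; Otherwise it maps the absolute input with a clamped range between the minimum and maximum shake amounts, adds the result to the running total and refreshes the UI.
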(event Custom|Shake
  (params (addShake :type Float%20%28double-precision%29))
  ;[1 1 1] Add shake value
  (if (> (Utilities|Map|Length (Variables|Default|Getingredient)) 0)
    (Variables|Default|SetshakeValue (+ (Math|Float|MapRangeClamped (Math|Float|Absolute(Float) addShake) 0.0 1e+02 (Variables|Default|GetminShake) (Variables|Default|GetmaxShake)) (Variables|Default|GetshakeValue)))
    (CallFunction|UpdateUI)))

(event EventBeginPlay
  (|CallParentFunction) ; This node is disabled and will not be called.\nDrag off pins to build functionality.
)

(fn ConstructionScript
  (|CallParentFunction))