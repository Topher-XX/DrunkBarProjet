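; First-person player Blueprint that handles movement, camera look and interacting with world objects through Enhanced Input.
; Interact line-traces forward from the camera and calls OnInteractEvent on the hit actor's ACS_Interact component, passing HandLoc as the hand.
; Cancel reuses the trace to teleport the actor attached to HandLoc to the impact point, then calls its OnCancelEvent; it requires a hit actor.
; The shared trace uses the Visibility channel and leaves debug drawing on.
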(event Input|EnhancedActionEvents|EnhancedInputActionIA_Move
  (params (ActionValue :type Vector%202D%20Structure) (ElapsedSeconds :type Float%20%28double-precision%29) (TriggeredSeconds :type Float%20%28double-precision%29) (InputAction :type Input%20Action%20Object%20Reference :default "/Game/_ProjetFiles/_Core/Inputs/IA_Move.IA_Move"))
  ;[0 1 0] Movements
  (:Triggered
    (Pawn|Input|AddMovementInput (* (Transformation|GetActorForwardVector) (.X (Math|Vector2D|BreakVector2D ActionValue))) (Variables|Default|GetmoveSpeed) false)
    (Pawn|Input|AddMovementInput (* (Transformation|GetActorRightVector) (.Y (Math|Vector2D|BreakVector2D ActionValue))) (Variables|Default|GetmoveSpeed) false)))

(event Input|EnhancedActionEvents|EnhancedInputActionIA_Look
  (params (ActionValue :type Vector%202D%20Structure) (ElapsedSeconds :type Float%20%28double-precision%29) (TriggeredSeconds :type Float%20%28double-precision%29) (InputAction :type Input%20Action%20Object%20Reference :default "/Game/_ProjetFiles/_Core/Inputs/IA_Look.IA_Look"))
  (bind (_x _y) (Math|Vector2D|BreakVector2D ActionValue))
  ;[0 1 0] Look
  (:Triggered
    (Pawn|Input|AddControllerYawInput _x)
    (Pawn|Input|AddControllerPitchInput _y)))

(event Input|EnhancedActionEvents|EnhancedInputActionIA_Interact
  (params (ActionValue :type Boolean) (ElapsedSeconds :type Float%20%28double-precision%29) (TriggeredSeconds :type Float%20%28double-precision%29) (InputAction :type Input%20Action%20Object%20Reference :default "/Game/_ProjetFiles/_Core/Inputs/IA_Interact.IA_Interact"))
  ;[0 1 0] Interact
  (:Started
    (bind _hitactor (CallFunction|LineTraceForwardCamera))
    (Utilities|IsValid _hitactor
      (:Is%20Valid
        (Utilities|IsValid (Actor|GetComponentbyClass _hitactor "/Game/_ProjetFiles/_Core/ACS/ACS_Interact.ACS_Interact_C")
          (:Is%20Valid
            (Default|OnInteractEvent (Actor|GetComponentbyClass _hitactor "/Game/_ProjetFiles/_Core/ACS/ACS_Interact.ACS_Interact_C") true (Variables|Default|GethandLoc))))))))

(event Input|EnhancedActionEvents|EnhancedInputActionIA_Cancel
  (params (ActionValue :type Boolean) (ElapsedSeconds :type Float%20%28double-precision%29) (TriggeredSeconds :type Float%20%28double-precision%29) (InputAction :type Input%20Action%20Object%20Reference :default "/Game/_ProjetFiles/_Core/Inputs/IA_Cancel.IA_Cancel"))
  (bind _handloc (Variables|Default|GethandLoc))
  (bind _returnvalue (Components|GetChildComponent _handloc 0))
  (bind _returnvalue_2 (Components|GetOwner _returnvalue))
  (bind _returnvalue_3 (Actor|GetComponentbyClass _returnvalue_2 "/Game/_ProjetFiles/_Core/ACS/ACS_Interact.ACS_Interact_C"))
  ;[0.004 1 0] Cancel
  (:Started
    (Utilities|IsValid _returnvalue
      (:Is%20Valid
        (bind (_hitactor _impactpoint) (CallFunction|LineTraceForwardCamera))
        (Utilities|IsValid _hitactor
          (:Is%20Valid
            (Utilities|IsValid _returnvalue_3
              (:Is%20Valid
                (Transformation|SetActorLocation _returnvalue_2 _impactpoint false true)
                (Default|OnCancelEvent _returnvalue_3)))))))))

(event EventBeginPlay)

(fn ConstructionScript)

(fn LineTraceForwardCamera
  (bind _camera (Variables|Default|GetCamera))
  (bind _returnvalue (Transformation|GetWorldLocation _camera))
  (bind _outhit (Collision|LineTraceByChannel _returnvalue (+ _returnvalue (* (Math|Vector|GetForwardVector (Variables|Default|GetCamera)) (Variables|Default|GetinteractRange))) "TraceTypeQuery1" false 0 "ForDuration"))
  (return (.HitActor (Collision|BreakHitResult _outhit)) (.Location (Collision|BreakHitResult _outhit))))