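; Player controller for a barman game that runs the day timer, the HUD, the end-of-day summary and pausing.
; BeginPlay adds the input mapping, creates the widgets and starts a timer that opens the summary when the day ends.
; The summary reads savings and salary from the ACSMoney component, with rent computed as half the savings; hiding it resets daily money.
; The pause action lazily creates its menu and toggles pause, cursor and input mode.
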(event Custom|ShowEndDayUI
  (bind _acs_money (Variables|Default|GetACS_Money))
  (UserInterface|Viewport|AddtoViewport (Variables|Default|GetendDayUI) 0)
  (Variables|Default|SetbShowMouseCursor true)
  (Default|SetSavings (Variables|Default|GetendDayUI) (Utilities|Text|ToText(Float) (Variables|/Game/_ProjetFiles/_Core/ACS/ACS_Money.ACS_Money_C|GetmoneyStock _acs_money) "HalfToEven"))
  (Default|SetSalary (Variables|Default|GetendDayUI) (Utilities|Text|ToText(Float) (Variables|/Game/_ProjetFiles/_Core/ACS/ACS_Money.ACS_Money_C|GetmoneyGainOnDay _acs_money) "HalfToEven"))
  (Default|SetRent (Variables|Default|GetendDayUI) (Utilities|Text|ToText(Float) (* (Variables|/Game/_ProjetFiles/_Core/ACS/ACS_Money.ACS_Money_C|GetmoneyStock (Variables|Default|GetACS_Money)) 0.5) "HalfToEven")))

(event Custom|HideEndDayUI
  (Widget|RemovefromParent (Variables|Default|GetendDayUI))
  (Variables|Default|SetbShowMouseCursor false)
  (Default|ResetMoneyDayEvent (Variables|Default|GetACS_Money)))

(event Custom|UpdateACSMoney
  (params (moneyToAdd :type Float%20%28double-precision%29))
  (Default|GiveMoneyEvent (Variables|Default|GetACS_Money) moneyToAdd))

(event Custom|StartDayTimer
  (Utilities|Time|SetTimerbyEvent (delegate Custom|EndDay) (Variables|Default|GetDayTime))
  (Variables|Default|SetisDay true))

(event Custom|EndDay
  (Variables|Default|SetisDay false)
  (CallFunction|ShowEndDayUI))

(event Input|EnhancedActionEvents|EnhancedInputActionIA_Pause
  (params (ActionValue :type Boolean) (ElapsedSeconds :type Float%20%28double-precision%29) (TriggeredSeconds :type Float%20%28double-precision%29) (InputAction :type Input%20Action%20Object%20Reference :default "/Game/FirstPerson/Input/Actions/IA_Pause.IA_Pause"))
  (bind _returnvalue (Game|GetPlayerController 0))
  (bind _returnvalue_2 (Game|GetPlayerController 0))
  ;[1 1 1] Pause game
  (:Started
    (Utilities|IsValid (Variables|Default|GetPauseRef)
      (:Is%20Valid
        _)
      (:Is%20Not%20Valid
        (bind _returnvalue_3 (UserInterface|CreateWidget "/Game/Menus/WB_Pause.WB_Pause_C"))
        (Variables|Default|SetPauseRef _returnvalue_3)))
    (if (Game|IsGamePaused)
      (Widget|RemovefromParent (Variables|Default|GetPauseRef))
      (Game|SetGamePaused false)
      (Variables|/Script/Engine.PlayerController|SetbShowMouseCursor _returnvalue false)
      (Input|SetInputModeGameOnly _returnvalue false)
      (else
        (UserInterface|Viewport|AddtoViewport (Variables|Default|GetPauseRef) 0)
        (Game|SetGamePaused true)
        (Variables|/Script/Engine.PlayerController|SetbShowMouseCursor _returnvalue_2 true)
        (Input|SetInputModeGameandUI _returnvalue_2 (Variables|Default|GetPauseRef) "DoNotLock" true false)))))

(event EventBeginPlay
  (Input|AddMappingContext (PlayerController|LocalPlayerSubsystems|GetEnhancedInputLocalPlayerSubsystem) "/Game/_ProjetFiles/_Core/Inputs/IMC_Barman.IMC_Barman" 0 "(bIgnoreAllPressedKeysUntilRelease=True,bForceImmediately=False,bNotifyUserSettings=False)")
  (bind _returnvalue (UserInterface|CreateWidget "/Game/_ProjetFiles/_Core/Widgets/WBP_PlayerInterface.WBP_PlayerInterface_C"))
  (bind _output_get (Variables|Default|SetplayerInterface _returnvalue))
  (UserInterface|Viewport|AddtoViewport _output_get 0)
  (bind _returnvalue_2 (UserInterface|CreateWidget "/Game/Menus/WB_EndOfDay.WB_EndOfDay_C"))
  (Variables|Default|SetendDayUI _returnvalue_2)
  (CallFunction|StartDayTimer))

(fn ConstructionScript)